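; BP_Building2 is a building obstacle Blueprint that labels itself with its size in meters.
; The construction script runs the parent script, then UpdateTextDepth writes the actor's X scale to TextRenderDepth as a height followed by "M".
; It resets the text's world scale to one so the label stays undistorted when the building is scaled.
; The event graph holds only disabled placeholder events.
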(fn `UpdateTextDepth`
  (bind _returnvalue_x (`KismetMathLibrary.BreakVector` (`self.GetActorScale3D`)))
  (`TextRenderComponent.K2_SetText` (`self.TextRender_Depth`) (`|FormatText` "{Height} M" (`KismetTextLibrary.Conv_DoubleToText` _returnvalue_x "HalfToEven")))
  (`SceneComponent.SetWorldScale3D` (`self.TextRender_Depth`) (1.0 1.0 1.0)))

(fn `UserConstructionScript`
  (`parent.UserConstructionScript`)
  (`self.UpdateTextDepth`))