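; BP_JumpMetricGuide is a level design guide that draws a predicted jump arc as a spline from the actor's location and orientation.
; The construction script traces a projectile path using fixed forward and up launch speeds, with gravity scaled by GravityScale.
; It then rebuilds the spline from the predicted points, so the arc updates whenever construction reruns.
; The event graph has no runtime logic.
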(event `self.ReceiveTick`
  (params (DeltaSeconds :type "Float (single-precision)")))

(fn `UserConstructionScript`
  (bind (_outhit _outpathpositions) (`GameplayStatics.Blueprint_PredictProjectilePath_ByTraceChannel` :`StartPos` (`self.K2_GetActorLocation`) :`LaunchVelocity` (+ (* (`self.GetActorForwardVector`) 1200.0) (* (`self.GetActorUpVector`) 420.0)) :`bTracePath` true :`TraceChannel` "ECC_Visibility" :`DrawDebugTime` 0.0 :`MaxSimTime` 5.0 :`OverrideGravityZ` (* (`self.GravityScale`) -900.0)))
  (`SplineComponent.ClearSplinePoints` (`self.Spline`) true)
  (for _array_element _outpathpositions
    (`SplineComponent.AddSplinePoint` (`self.Spline`) _array_element "World" true)))