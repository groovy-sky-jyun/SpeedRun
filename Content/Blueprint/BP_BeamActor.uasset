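; BP_BeamActor is a spline-driven actor that builds a beam from spline mesh segments, with no active event logic.
; The construction script divides the spline length by MeshLength, adding a spline mesh with the set Material for each segment.
; GetSplineStartAndEnd samples local location and normalized tangent at index times MeshLength, so neighboring segments share endpoints along the curve.
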(fn `GetSplineStartAndEnd`
  (params (A :type Integer))
  (returns (Location :type "Vector Structure") (Tangent :type "Vector Structure"))
  (bind _spline (`self.Spline`))
  (bind _returnvalue (* A (`self.MeshLength`)))
  (return (`SplineComponent.GetLocationAtDistanceAlongSpline` _spline _returnvalue "Local") (`KismetMathLibrary.Normal` (`SplineComponent.GetTangentAtDistanceAlongSpline` _spline _returnvalue "Local"))))

(fn `UserConstructionScript`
  (for _index (range (+ (`KismetMathLibrary.FTrunc` (/ (`SplineComponent.GetSplineLength` (`self.Spline`)) (`self.MeshLength`))) 1))
    (bind _returnvalue (`AddComponent|NODE_AddSplineMeshComponent-0`))
    (`PrimitiveComponent.SetMaterial` _returnvalue 0 (`self.Material`))
    (`SceneComponent.K2_AttachToComponent` _returnvalue (`self.DefaultSceneRoot`) "None" "KeepRelative" "KeepRelative" "KeepRelative" true)
    (bind (_location _tangent) (`self.GetSplineStartAndEnd` _index))
    (bind (_location_2 _tangent_2) (`self.GetSplineStartAndEnd` (+ _index 1)))
    (`SplineMeshComponent.SetStartAndEnd` _returnvalue _location _tangent _location_2 _tangent_2 true)
    (set `SplineComponent.bInputSplinePointsToConstructionScript` true (`self.Spline`))))